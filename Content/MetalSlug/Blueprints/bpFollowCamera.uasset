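; Side-scrolling follow camera for the Metal Slug game that tracks the player along X and never scrolls backward.
; Each Tick it copies last and max X from MarkoRossiCharacter, moving only when the player passes the last and reaches the max.
; The move uses TInterpTo with fixed rotation and a world offset.
; The interpolation's start already uses the player's X, so horizontal motion snaps rather than eases.
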(event `self.ReceiveTick`
  (params (DeltaSeconds :type "Float (single-precision)"))
  (bind _returnvalue (`GameplayStatics.GetPlayerPawn` 0))
  (`/Engine/EditorBlueprintResources/StandardMacros.IsValid` _returnvalue
    (:`Is Valid`
      (bind _asmarko_rossi_character (cast `/Game/MetalSlug/Blueprints/MarkoRossiCharacter` (`GameplayStatics.GetPlayerCharacter` 0)))
      (bind _output_get (set `self.camerasPlayrLastX` (`/Game/MetalSlug/Blueprints/MarkoRossiCharacter.playersLastX` _asmarko_rossi_character)))
      (bind _output_get_2 (set `self.camerasPlayrMaxX` (`/Game/MetalSlug/Blueprints/MarkoRossiCharacter.playersMaxX` _asmarko_rossi_character)))
      (if (and (> (.x (.location (`self.GetTransform` _returnvalue))) _output_get) (>= (.x (.location (`self.GetTransform` _returnvalue))) _output_get_2))
        (`self.K2_SetActorTransform` (`KismetMathLibrary.TInterpTo` (`KismetMathLibrary.MakeTransform` (+ (`KismetMathLibrary.MakeVector` (.x (.location (`self.GetTransform` _returnvalue))) (.y (.location (`self.GetTransform`))) (.z (.location (`self.GetTransform`)))) (`self.WorldOffset`)) (struct :`Yaw` -90.0)) (`KismetMathLibrary.MakeTransform` (`KismetMathLibrary.MakeVector` (.x (+ (.location (`self.GetTransform` _returnvalue)) (`self.WorldOffset`))) (.y (+ (.location (`self.GetTransform` _returnvalue)) (`self.WorldOffset`))) (.z (.location (`self.GetTransform`)))) (struct :`Yaw` -90.0)) (`GameplayStatics.GetWorldDeltaSeconds`) 20.0))))))

(fn `UserConstructionScript`)